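; BP_Plus is a collectible pickup that awards a point to the player character.
; On BeginPlay it gives itself a random rotation on all three axes.
; When its Sphere component overlaps a BP_Char, it calls AddPoint on that character, plays a sound at its location and destroys itself.
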(event OnComponentBeginOverlap(Sphere)
  (params (OverlappedComponent :type Primitive%20Component%20Object%20Reference) (OtherActor :type Actor%20Object%20Reference) (OtherComp :type Primitive%20Component%20Object%20Reference) (OtherBodyIndex :type Integer) (bFromSweep :type Boolean) (SweepResult :type Hit%20Result%20Structure%20%28by%20ref%29))
  (bind _asbp_char (Utilities|Casting|CastToBP_Char OtherActor))
  (Default|AddPoint _asbp_char)
  (Audio|SpawnSoundatLocation (Variables|Default|Getsound) (Transformation|GetActorLocation))
  (Actor|DestroyActor))

(event EventBeginPlay
  (Transformation|SetActorRotation (Math|Rotator|MakeRotator (Math|Random|RandomFloatinRange -9e+01 9e+01) (Math|Random|RandomFloatinRange -9e+01 9e+01) (Math|Random|RandomFloatinRange -9e+01 9e+01))))

(fn ConstructionScript)