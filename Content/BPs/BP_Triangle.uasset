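; BP_Triangle is an actor that temporarily changes the player character's FallingSpeed when BP_Char overlaps its sphere.
; The IsReverse flag selects between a fixed speed and a tiered one chosen by the SuperBoost and MediumBoost flags.
; Both paths play the slowdown sound at the actor's location, then a three-second delay resets FallingSpeed to a hardcoded base value.
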(event OnComponentBeginOverlap(Sphere)
  (params (OverlappedComponent :type Primitive%20Component%20Object%20Reference) (OtherActor :type Actor%20Object%20Reference) (OtherComp :type Primitive%20Component%20Object%20Reference) (OtherBodyIndex :type Integer) (bFromSweep :type Boolean) (SweepResult :type Hit%20Result%20Structure%20%28by%20ref%29))
  (bind _returnvalue (Transformation|GetActorLocation))
  (bind _slowdownsounds (Variables|Default|Getslowdownsounds))
  (bind _asbp_char (Utilities|Casting|CastToBP_Char OtherActor))
  (if (Variables|Default|GetisReverse)
    (if (Variables|Default|GetsuperBoost)
      (Variables|/Game/BPs/BP_Char.BP_Char_C|SetfallingSpeed _asbp_char 4e+01)
      (elif (Variables|Default|GetmediumBoost)
        (Variables|/Game/BPs/BP_Char.BP_Char_C|SetfallingSpeed _asbp_char 3e+01)
        (else
          (Variables|/Game/BPs/BP_Char.BP_Char_C|SetfallingSpeed _asbp_char 2e+01))))
    (Audio|SpawnSoundatLocation _slowdownsounds _returnvalue)
    (else
      (Variables|/Game/BPs/BP_Char.BP_Char_C|SetfallingSpeed _asbp_char 1e+01)
      (Audio|SpawnSoundatLocation _slowdownsounds _returnvalue)))
  (Utilities|FlowControl|Delay 3.0)
  (Variables|/Game/BPs/BP_Char.BP_Char_C|SetfallingSpeed _asbp_char 7.0))

(fn ConstructionScript)