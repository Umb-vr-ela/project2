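; End-of-game menu actor that moves to the player on spawn, showing a score leaderboard and a gaze-operated restart button.
; BeginPlay loads the SaveScore slot, inserts BP_Char's total points by rank, fills the leaderboard widget and saves the list.
; Tick traces from the camera, filling the button's progress while looked at and draining it otherwise.
; A two-second dwell streams in Level_Island and destroys the menu.
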(event EventBeginPlay
  (bind _array (Variables|Default|GetArray))
  (Transformation|SetActorLocation (Transformation|GetActorLocation (Game|Player|GetPlayerPawn 0)) false false)
  (Transformation|SetActorRotation "0,90.000000, 0")
  (Utilities|FlowControl|DoOnce false
    (:Completed
      (bind _returnvalue (SaveGame|LoadGamefromSlot "SaveScore"))
      (bind _assave_score (Utilities|Casting|CastToSaveScore _returnvalue)
        (:then
          (for _array_element (Variables|/Game/Leaderboard/SaveScore.SaveScore_C|GetPlayerScores _assave_score)
            (Utilities|Array|Add _array _array_element))
          (Utilities|FlowControl|Sequence :!label _label
            (:then_0
              (Utilities|FlowControl|DoOnce false :!label _label_2
                (:Completed
                  (CallFunction|AddScore))))
            (:then_1
              (bind _returnvalue_2 (UserInterface|CreateWidget "/Game/Widgets/LeaderboardInterface.LeaderboardInterface_C" 0 _array))
              (UserInterface|SetWidget (Variables|Default|GetLeaderboard) _returnvalue_2))
            (:then_2
              (bind _returnvalue_3 (SaveGame|CreateSaveGameObject "/Game/Leaderboard/SaveScore.SaveScore_C"))
              (Variables|/Game/Leaderboard/SaveScore.SaveScore_C|SetPlayerScores _returnvalue_3 _array)
              (SaveGame|SaveGametoSlot _returnvalue_3 "SaveScore"))))
        (:CastFailed
          (Utilities|FlowControl|Sequence
            (:then_0
              (goto _label_2))
            (:then_1
              (goto _label))))))))

(event EventTick
  (params (DeltaSeconds :type Float%20%28single-precision%29))
  (bind _restartbutton (Variables|Default|GetRestartButton))
  (if (>= (Variables|Default|GetdeltaTime) 2.0)
    (Game|LoadStreamLevel(byName) "Level_Island" true)
    (Actor|DestroyActor)
    (else
      (bind _asbp_char (Utilities|Casting|CastToBP_Char (Game|GetPlayerCharacter 0)))
      (bind _outhit (Collision|LineTraceByChannel (Transformation|GetWorldLocation (Variables|/Game/BPs/BP_Char.BP_Char_C|GetCamera _asbp_char)) (+ (* (Math|Vector|GetForwardVector (Variables|/Game/BPs/BP_Char.BP_Char_C|GetCamera _asbp_char)) 1e+05) (Transformation|GetWorldLocation (Variables|/Game/BPs/BP_Char.BP_Char_C|GetCamera _asbp_char))) "TraceTypeQuery1" false 0 "None" false "(R=1.000000,G=0.000000,B=0.000000,A=1.000000)" "(R=0.000000,G=1.000000,B=0.000000,A=1.000000)" 0.0))
      (if (== (.HitComponent (Collision|BreakHitResult _outhit)) _restartbutton)
        (Variables|Default|SetdeltaTime (+ (Variables|Default|GetdeltaTime) DeltaSeconds))
        (elif (>= (- (Variables|Default|GetdeltaTime) DeltaSeconds) 0.0)
          (Variables|Default|SetdeltaTime (- (Variables|Default|GetdeltaTime) DeltaSeconds))
          (else
            (Variables|Default|SetdeltaTime 0.0))))
      (bind _asgame_over_interface_button (Utilities|Casting|CastToGameOverInterface_Button (UserInterface|GetUserWidgetObject _restartbutton)))
      (Default|SetPercentage _asgame_over_interface_button (/ (Variables|Default|GetdeltaTime) 2.0)))))

(fn ConstructionScript)

(fn AddScore
  (bind _array (Variables|Default|GetArray))
  (bind _asbp_char (Utilities|Casting|CastToBP_Char (Game|GetPlayerCharacter 0)))
  (bind (_array_element _array_index) (Utilities|Array|ForEachLoopwithBreak _array :!label _label)
    (:LoopBody
      (if (> (Variables|/Game/BPs/BP_Char.BP_Char_C|GettotalPoints _asbp_char) (.Score (Utilities|Struct|BreakPlayerScore _array_element)))
        (Utilities|Array|Insert _array (Utilities|Struct|MakePlayerScore "Name" (Variables|/Game/BPs/BP_Char.BP_Char_C|GettotalPoints _asbp_char)) _array_index :!label _label_2)
        (goto _label Break)))
    (:Completed
      (if (not (Utilities|Array|ContainsItem _array (Utilities|Struct|MakePlayerScore "Name" (Variables|/Game/BPs/BP_Char.BP_Char_C|GettotalPoints _asbp_char))))
        (goto _label_2)))))