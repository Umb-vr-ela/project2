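; BP_Cloud is a Blueprint that scatters cloud particle effects when play begins.
; A loop on BeginPlay repeatedly attaches P_Cloud_Lit2 emitters to the Clouds component at random horizontal offsets within Range and random heights, then doubles their world scale.
; A random three-way switch has no effect on the emitter chosen, as the Lit3 and Lit4 spawn branches are disconnected and never run.
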(event EventBeginPlay
  (bind _range (Variables|Default|Getrange))
  (bind _returnvalue (* _range -1))
  (for _index (range 0 25)
    (switch int (Math|Random|RandomInteger 3)
      (:0
        _)
      (:1
        _)
      (:2
        _))
    (bind _returnvalue_2 (Effects|SpawnEmitterAttached "/Game/Particles/P_Cloud_Lit2.P_Cloud_Lit2" (Variables|Default|GetClouds) "None" (Math|Vector|MakeVector (Math|Conversions|ToFloat(Integer) (Math|Random|RandomIntegerinRange _returnvalue _range)) (Math|Conversions|ToFloat(Integer) (Math|Random|RandomIntegerinRange _returnvalue _range)) (Math|Conversions|ToFloat(Integer) (Math|Random|RandomIntegerinRange 0 20000)))))
    (Transformation|SetWorldScale3D _returnvalue_2 "2.000000,2.000000,2.000000")))

(fn ConstructionScript)