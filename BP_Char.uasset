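; Google VR player character that moves by controller tilt, carries an umbrella, and tracks points and health.
; Tick reads raw controller acceleration to tilt the umbrella and, within range thresholds, drive movement along the controller's axes.
; While door checking is on, a camera trace destroys an actor named "door", then enables movement after a delay.
; The complementary filter is never called, the computed angle is unused, and zero health only prints "Game Over".
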(event Custom|checkUmbrellaRotation
  (bind _returnvalue (Class|GoogleVRControllerFunctionLibrary|GetGoogleVRControllerRawAccel))
  (bind (_x _y) (Math|Vector|BreakVector _returnvalue))
  (Transformation|SetRelativeRotation (Variables|Default|Getumbrella) (Math|Rotator|MakeRotator (* _x -9.0) (* _y -9.0) 0.0) false false))

(event Custom|CheckDoors
  (if (Variables|Default|GetcheckForDoor)
    (bind _result (CallFunction|LinetraceDoor))
    (if _result
      (Utilities|FlowControl|Delay 2.0)
      (Variables|Default|SetmovementEnabled true))))

(event Custom|checkMovement
  (bind _returnvalue (Class|GoogleVRControllerFunctionLibrary|GetGoogleVRControllerRawAccel))
  (bind _minrange (Variables|Default|GetminRange))
  (bind _maxrange (Variables|Default|GetmaxRange))
  (bind _move_speed (Variables|Default|Getmove%20speed))
  (bind _googlevrmotioncontroller (Variables|Default|GetGoogleVRMotionController))
  (bind (_x _y) (Math|Vector|BreakVector _returnvalue))
  (bind _returnvalue_2 (Math|Vector|GetRightVector _googlevrmotioncontroller))
  (bind _returnvalue_3 (Math|Vector|GetForwardVector _googlevrmotioncontroller))
  (bind _returnvalue_4 (* -1 _move_speed))
  (bind _returnvalue_5 (* _maxrange -1.0))
  (bind _returnvalue_6 (* _minrange -1.0))
  (if (Variables|Default|GetmovementEnabled)
    (Variables|Default|Setforward (Math|Float|InRange(Float) _y _minrange _maxrange))
    (Variables|Default|Setback (Math|Float|InRange(Float) _y _returnvalue_5 _returnvalue_6))
    (Variables|Default|Setright (Math|Float|InRange(Float) _x _minrange _maxrange))
    (Variables|Default|Setleft (Math|Float|InRange(Float) _x _returnvalue_5 _returnvalue_6))
    (if (Variables|Default|Getforward)
      (Pawn|Input|AddMovementInput _returnvalue_3 1.0 false))
    (if (Variables|Default|Getback)
      (Pawn|Input|AddMovementInput _returnvalue_3 _returnvalue_4 false))
    (if (Variables|Default|Getleft)
      (Pawn|Input|AddMovementInput _returnvalue_2 _move_speed false))
    (if (Variables|Default|Getright)
      (Pawn|Input|AddMovementInput _returnvalue_2 _returnvalue_4 false))))

(event EventTick
  (params (DeltaSeconds :type Float%20%28single-precision%29))
  (Variables|Default|SetDelta%20Time DeltaSeconds)
  (Variables|Default|SetCompFilter%20B (- 1.0 (Variables|Default|GetCompFilter%20A)))
  (bind _angle (CallFunction|GetAngle (Math|Vector|GetRightVector (Variables|Default|GetGoogleVRMotionController)) (Math|Vector|GetRightVector (Variables|Default|GetGoogleVRMotionController))))
  (CallFunction|CheckDoors)
  (CallFunction|CheckMovement)
  (CallFunction|CheckUmbrellaRotation))

(fn ConstructionScript)

(fn AddPoint
  (Variables|Default|SettotalPoints (+ (Variables|Default|GettotalPoints) 1)))

(fn LinetraceDoor
  (bind _camera (Variables|Default|GetCamera))
  (bind _returnvalue (Transformation|GetWorldLocation _camera))
  (bind _outhit (Collision|LineTraceByChannel _returnvalue (+ _returnvalue (* (Math|Vector|GetForwardVector _camera) 1e+04)) "TraceTypeQuery1" false 0 "None"))
  (if (Utilities|String|Contains (Utilities|GetDisplayName (.HitActor (Collision|BreakHitResult _outhit))) "door")
    (Actor|DestroyActor (.HitActor (Collision|BreakHitResult _outhit)))
    (Variables|Default|SetcheckForDoor false)
    (return true)))

(fn ReduceHealth
  (bind _output_get (Variables|Default|Sethealth (- (Variables|Default|Gethealth) 1)))
  (if (<= (- (Variables|Default|Gethealth) 1) 0)
    (Development|PrintString "Game Over")
    (else
      (Development|PrintString (Utilities|String|ToString(Integer) _output_get)))))

(fn GetAngle
  (params (vec1 :type Vector) (vec2 :type Vector))
  (return (Class|KismetMathLibrary|DegAcos (Math|Vector|DotProduct (Math|Vector|Normalize vec1) (Math|Vector|Normalize vec2)))))

(fn ComplementaryFilter
  (params (RawGyro :type Vector))
  (bind _returnvalue (Class|GoogleVRControllerFunctionLibrary|GetGoogleVRControllerRawAccel))
  (bind _delta_time (Variables|Default|GetDelta%20Time))
  (bind _returnvalue_2 (* _returnvalue _delta_time))
  (bind (_x _y) (Math|Vector|BreakVector _returnvalue_2))
  (return (+ (* (+ _returnvalue_2 (Class|KismetMathLibrary|DegAtan2 _x _y)) (Variables|Default|GetCompFilter%20A)) (* RawGyro (Variables|Default|GetCompFilter%20B)))))