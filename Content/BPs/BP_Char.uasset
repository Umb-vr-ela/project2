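; Player character for a Google VR game that falls while holding an umbrella, steered by tilting the motion controller.
; Each tick lowers the actor with a sweep, maps raw controller acceleration within thresholds to horizontal movement, and tilts the umbrella to match.
; Functions handle points, health with a printed game over, pausing fall and movement, and showing snow particles.
; Angle, complementary filter and rotation helpers are defined but not called here.
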(event Custom|checkUmbrellaRotation
  (bind _returnvalue (Class|GoogleVRControllerFunctionLibrary|GetGoogleVRControllerRawAccel))
  (bind (_x _y) (Math|Vector|BreakVector _returnvalue))
  (Transformation|SetRelativeRotation (Variables|Default|Getumbrella) (Math|Rotator|MakeRotator (* _x -9.0) (* _y -9.0) 0.0) false false))

(event Custom|falling
  (bind _returnvalue (Transformation|GetActorLocation))
  (bind (_x _y _z) (Math|Vector|BreakVector _returnvalue))
  (Transformation|SetActorLocation (Math|Vector|MakeVector _x _y (- _z (Variables|Default|GetfallingSpeed))) true false))

(event Custom|checkMovement
  (bind _returnvalue (Class|GoogleVRControllerFunctionLibrary|GetGoogleVRControllerRawAccel))
  (bind _googlevrmotioncontroller (Variables|Default|GetGoogleVRMotionController))
  (bind _horizontalspeed (Variables|Default|GethorizontalSpeed))
  (bind _umbrellaminrange (Variables|Default|GetumbrellaMinRange))
  (bind _umbreallamaxrange (Variables|Default|GetUmbreallaMaxRange))
  (bind (_x _y) (Math|Vector|BreakVector _returnvalue))
  (bind _returnvalue_2 (Math|Vector|GetRightVector _googlevrmotioncontroller))
  (bind _returnvalue_3 (Math|Vector|GetForwardVector _googlevrmotioncontroller))
  (bind _returnvalue_4 (* -1 _horizontalspeed))
  (bind _returnvalue_5 (* _umbreallamaxrange -1.0))
  (bind _returnvalue_6 (* _umbrellaminrange -1.0))
  (if (Variables|Default|GetmovementEnabled)
    (Variables|Default|Setforward (Math|Float|InRange(Float) _y _umbrellaminrange _umbreallamaxrange))
    (Variables|Default|Setback (Math|Float|InRange(Float) _y _returnvalue_5 _returnvalue_6))
    (Variables|Default|Setright (Math|Float|InRange(Float) _x _umbrellaminrange _umbreallamaxrange))
    (Variables|Default|Setleft (Math|Float|InRange(Float) _x _returnvalue_5 _returnvalue_6))
    (if (Variables|Default|Getforward)
      (Pawn|Input|AddMovementInput _returnvalue_3 _horizontalspeed false))
    (if (Variables|Default|Getback)
      (Pawn|Input|AddMovementInput _returnvalue_3 _returnvalue_4 false))
    (if (Variables|Default|Getleft)
      (Pawn|Input|AddMovementInput _returnvalue_2 _horizontalspeed false))
    (if (Variables|Default|Getright)
      (Pawn|Input|AddMovementInput _returnvalue_2 _returnvalue_4 false))))

(event EventTick
  (params (DeltaSeconds :type Float%20%28single-precision%29))
  (CallFunction|Falling)
  (CallFunction|CheckMovement)
  (CallFunction|CheckUmbrellaRotation))

(fn ConstructionScript)

(fn AddPoint
  (Variables|Default|SettotalPoints (+ (Variables|Default|GettotalPoints) 1)))

(fn ReduceHealth
  (bind _output_get (Variables|Default|Sethealth (- (Variables|Default|Gethealth) 1)))
  (if (<= (- (Variables|Default|Gethealth) 1) 0)
    (Development|PrintString "Game Over")
    (else
      (Development|PrintString (Utilities|String|ToString(Integer) _output_get)))))

(fn GetAngle
  (params (vec1 :type Vector) (vec2 :type Vector))
  (return (Class|KismetMathLibrary|DegAcos (Math|Vector|DotProduct (Math|Vector|Normalize vec1) (Math|Vector|Normalize vec2)))))

(fn ComplementaryFilter
  (params (RawAccel :type Vector))
  (bind _returnvalue (Class|GoogleVRControllerFunctionLibrary|GetGoogleVRControllerRawGyro))
  (bind (_x _y) (Math|Vector|BreakVector _returnvalue))
  (return (+ (* (+ (* _returnvalue (Variables|Default|GetDelta%20Time)) (Class|KismetMathLibrary|DegAtan2 _x _y)) (Variables|Default|GetCompFilter%20A)) (* RawAccel (Variables|Default|GetCompFilter%20B)))))

(fn XYRotationMatrix
  (params (theta :type Float%20%28single-precision%29) (X :type Float%20%28single-precision%29) (Y :type Float%20%28single-precision%29))
  (bind _returnvalue (Math|Trig|Cos(Radians) theta))
  (bind _returnvalue_2 (Math|Trig|Sin(Radians) theta))
  (return (- (* _returnvalue X) (* _returnvalue_2 Y)) (+ (* _returnvalue_2 X) (* _returnvalue Y))))

(fn SetMovement
  (params (isEnabled :type Boolean))
  (Variables|Default|SetmovementEnabled isEnabled)
  (if isEnabled
    (Variables|Default|SetfallingSpeed 7.0)
    (else
      (Variables|Default|SetfallingSpeed 0.0)
      (Components|Movement|StopMovementImmediately (Variables|Character|GetCharacterMovement)))))

(fn EnableSnow
  (Rendering|SetVisibility (Variables|Default|GetParticleSystem_snow) true false)
  (Rendering|SetVisibility (Variables|Default|GetParticleSystem) true false))