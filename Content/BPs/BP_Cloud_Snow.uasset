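; BP_Cloud_Snow is a cloud scattering actor that fills the sky with particle clouds when play begins.
; A single BeginPlay loop repeatedly picks one of three lit cloud emitter templates at random and attaches it to the Clouds component.
; Each emitter gets a random horizontal offset within Range and a random height in a tall fixed band, then a uniform enlarged scale.
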(event EventBeginPlay
  (bind _returnvalue (Math|Random|RandomIntegerinRange 2000 97503))
  (bind _clouds (Variables|Default|GetClouds))
  (bind _range (Variables|Default|Getrange))
  (bind _returnvalue_2 (Math|Conversions|ToFloat(Integer) _returnvalue))
  (bind _returnvalue_3 (* _range -1))
  (bind _returnvalue_4 (Math|Random|RandomIntegerinRange _returnvalue_3 _range))
  (bind _returnvalue_5 (Math|Random|RandomIntegerinRange _returnvalue_3 _range))
  (bind _returnvalue_6 (Math|Conversions|ToFloat(Integer) _returnvalue_4))
  (bind _returnvalue_7 (Math|Conversions|ToFloat(Integer) _returnvalue_5))
  (bind _returnvalue_8 (Math|Vector|MakeVector _returnvalue_6 _returnvalue_7 _returnvalue_2))
  (for _index (range 0 100)
    (switch int (Math|Random|RandomInteger 3)
      (:0
        (bind _returnvalue_9 (Effects|SpawnEmitterAttached "/Game/Particles/P_Cloud_Lit2.P_Cloud_Lit2" _clouds "None" _returnvalue_8))
        (Transformation|SetWorldScale3D _returnvalue_9 "8.000000,8.000000,8.000000"))
      (:1
        (bind _returnvalue_10 (Effects|SpawnEmitterAttached "/Game/Particles/P_Cloud_Lit3.P_Cloud_Lit3" _clouds "None" _returnvalue_8))
        (Transformation|SetWorldScale3D _returnvalue_10 "8.000000,8.000000,8.000000"))
      (:2
        (bind _returnvalue_11 (Effects|SpawnEmitterAttached "/Game/Particles/P_Cloud_Lit4.P_Cloud_Lit4" _clouds "None" _returnvalue_8))
        (Transformation|SetWorldScale3D _returnvalue_11 "8.000000,8.000000,8.000000")))))

(fn ConstructionScript)