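; Gaze-operated start menu actor that holds the player at game start until they look at the start button long enough.
; BeginPlay places the menu at a fixed offset from the player's eyes, unpauses the game and keeps both widgets tickable when paused.
; Tick line-traces from BP_Char's camera, filling or draining a dwell timer shown as button progress.
; A full timer enables player movement and destroys the menu.
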(event EventBeginPlay
  (bind _returnvalue (Game|Player|GetPlayerPawn 0))
  (bind _startmenuwidget (Variables|Default|GetStartMenuWidget))
  (bind _instructionswidget (Variables|Default|GetInstructionsWidget))
  (bind _returnvalue_2 (Components|GetOwner _startmenuwidget))
  (bind _outlocation (Actor|GetActorEyesViewPoint _returnvalue))
  (bind _returnvalue_3 (Components|GetOwner _instructionswidget))
  (bind _returnvalue_4 (+ _outlocation "-50.000000,300.000000,-50.000000"))
  (Transformation|SetActorRotation _returnvalue_2 "0,-90.000000, 0")
  (Transformation|SetActorLocation _returnvalue_2 _returnvalue_4 false false)
  (Transformation|SetActorRotation _returnvalue_3 "0,-90.000000, 0")
  (Transformation|SetActorLocation _returnvalue_3 _returnvalue_4 false false)
  (Game|SetGamePaused false)
  (Class|ActorComponent|SetTickablewhenPaused (Variables|Default|GetStartMenuWidget) true)
  (Class|ActorComponent|SetTickablewhenPaused (Variables|Default|GetInstructionsWidget) true))

(event EventTick
  (params (DeltaSeconds :type Float%20%28single-precision%29))
  (bind _returnvalue (Game|GetPlayerCharacter 0))
  (bind _startbutton (Variables|Default|GetStartButton))
  (if (>= (Variables|Default|GetdeltaTime) 3.0)
    (bind _asbp_char (Utilities|Casting|CastToBP_Char _returnvalue))
    (Default|EnableMovement _asbp_char)
    (Actor|DestroyActor)
    (else
      (bind _asbp_char_2 (Utilities|Casting|CastToBP_Char _returnvalue))
      (bind _outhit (Collision|LineTraceByChannel (Transformation|GetWorldLocation (Variables|/Game/BPs/BP_Char.BP_Char_C|GetCamera _asbp_char_2)) (+ (* (Math|Vector|GetForwardVector (Variables|/Game/BPs/BP_Char.BP_Char_C|GetCamera _asbp_char_2)) 1e+05) (Transformation|GetWorldLocation (Variables|/Game/BPs/BP_Char.BP_Char_C|GetCamera _asbp_char_2))) "TraceTypeQuery1" false 0 "None" false "(R=1.000000,G=0.000000,B=0.000000,A=1.000000)" "(R=0.000000,G=1.000000,B=0.000000,A=1.000000)" 0.0))
      (if (== (.HitComponent (Collision|BreakHitResult _outhit)) _startbutton)
        (Variables|Default|SetdeltaTime (+ (Variables|Default|GetdeltaTime) DeltaSeconds))
        (elif (>= (- (Variables|Default|GetdeltaTime) DeltaSeconds) 0.0)
          (Variables|Default|SetdeltaTime (- (Variables|Default|GetdeltaTime) DeltaSeconds))
          (else
            (Variables|Default|SetdeltaTime 0.0))))
      (bind _asstart_game_interface_button (Utilities|Casting|CastToStartGameInterface_Button (UserInterface|GetUserWidgetObject _startbutton)))
      (Default|SetPercentage _asstart_game_interface_button (/ (Variables|Default|GetdeltaTime) 3.0)))))

(fn ConstructionScript)