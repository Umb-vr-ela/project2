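; Volumetric cloud actor that rises straight up and destroys itself once it reaches a height limit.
; Construction applies a dynamic ray-march volume material to its static mesh, randomly choosing one of two cloud render textures.
; Each tick adds a vertical step that grows with the square root of game time, not actor age, up to a cap.
; The step ignores delta time, so climb rate depends on frame rate.
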(event Custom|CalculateSpeed
  (bind _returnvalue (Utilities|Time|GetTimeSeconds))
  (if (>= _returnvalue 36.0)
    (Variables|Default|SetspeedZ 18.0)
    (else
      (Variables|Default|SetspeedZ (* 3.0 (Math|Float|Sqrt _returnvalue)))))
  (Variables|Default|Setspeed (Math|Vector|MakeVector 0.0 0.0 (Variables|Default|GetspeedZ))))

(event EventTick
  (params (DeltaSeconds :type Float%20%28single-precision%29))
  (bind _returnvalue (Transformation|GetActorLocation))
  (if (>= (.Z (Math|Vector|BreakVector _returnvalue)) 1e+04)
    (Actor|DestroyActor)
    (else
      (CallFunction|CalculateSpeed)
      (Transformation|SetActorLocation (+ _returnvalue (Variables|Default|Getspeed)) false false))))

(fn ConstructionScript
  (bind _returnvalue (Rendering|Material|CreateDynamicMaterialInstance "/Game/Materials/M_VolumeRayMarch_Lit_LinearSteps.M_VolumeRayMarch_Lit_LinearSteps" :!class /Script/Engine.KismetMaterialLibrary))
  (switch int (Math|Random|RandomInteger 2)
    (:0
      (Rendering|Material|SetTextureParameterValue _returnvalue "CloudTex" "/Game/Textures/RT_Cloud_1.RT_Cloud_1"))
    (:1
      (Rendering|Material|SetTextureParameterValue _returnvalue "CloudTex" "/Game/Textures/RT_Cloud_2.RT_Cloud_2")))
  (Rendering|Material|SetMaterial (Variables|Default|GetStaticMesh) 0 _returnvalue))