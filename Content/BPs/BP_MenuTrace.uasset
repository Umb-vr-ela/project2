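; BP_MenuTrace is a Blueprint that reports what the player character's camera is looking at.
; Every tick it casts the player character to BP_Char and runs a long Visibility line trace forward from that camera, with debug drawing.
; It prints the hit actor's name to screen; despite the asset's name, no menu or widget logic is connected.
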(event EventBeginPlay)

(event Collision|EventActorBeginOverlap
  (params (OtherActor :type Actor%20Object%20Reference)))

(event EventTick
  (params (DeltaSeconds :type Float%20%28single-precision%29))
  (bind _asbp_char (Utilities|Casting|CastToBP_Char (Game|GetPlayerCharacter 0)))
  (bind _outhit (Collision|LineTraceByChannel (Transformation|GetWorldLocation (Variables|/Game/BPs/BP_Char.BP_Char_C|GetCamera _asbp_char)) (+ (* (Math|Vector|GetForwardVector (Variables|/Game/BPs/BP_Char.BP_Char_C|GetCamera _asbp_char)) 1e+05) (Transformation|GetWorldLocation (Variables|/Game/BPs/BP_Char.BP_Char_C|GetCamera _asbp_char))) "TraceTypeQuery1" false 0 "ForDuration"))
  (Development|PrintString (Utilities|GetDisplayName (.HitActor (Collision|BreakHitResult _outhit)))))

(fn ConstructionScript)