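; BP_VCloudGenerator is a spawner actor that continually adds volumetric clouds to the level.
; On BeginPlay it starts a looping one-second timer that calls spawnCloud.
; Each call spawns a double-scale BP_VolumetricCloud at random X and Y within fixed ranges and a fixed negative Z.
; Positions are absolute world coordinates, independent of the generator, and an unconnected player-location calculation is unused.
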(event Custom|spawnCloud
  (Game|SpawnActorfromClass "/Game/BPs/BP_VolumetricCloud.BP_VolumetricCloud_C" (Math|Transform|MakeTransform (Math|Vector|MakeVector (Math|Conversions|ToFloat(Integer) (Math|Random|RandomIntegerinRange -50 500)) (Math|Conversions|ToFloat(Integer) (Math|Random|RandomIntegerinRange -500 500)) -2e+02) "0, 0, 0" "2.000000,2.000000,2.000000") "Undefined" 0 0))

(event EventBeginPlay
  (Utilities|Time|SetTimerbyFunctionName 0 "spawnCloud" 1.0 true))

(event Collision|EventActorBeginOverlap
  (params (OtherActor :type Actor%20Object%20Reference)))

(event EventTick
  (params (DeltaSeconds :type Float%20%28single-precision%29)))

(fn ConstructionScript)