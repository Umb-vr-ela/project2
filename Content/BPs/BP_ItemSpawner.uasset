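; Item spawner segment that fills an area with items and asks the game mode for another spawner when the player passes through.
; On BeginPlay it adds several scaled-up child actors at random points inside the ItemArea box.
; When BP_Char overlaps EndTrigger, it calls AddSpawner on VR_GameMode, then destroys itself after a short delay.
; GetAttachTransform exposes the AttachPoint world transform.
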(event OnComponentBeginOverlap(EndTrigger)
  (params (OverlappedComponent :type Primitive%20Component%20Object%20Reference) (OtherActor :type Actor%20Object%20Reference) (OtherComp :type Primitive%20Component%20Object%20Reference) (OtherBodyIndex :type Integer) (bFromSweep :type Boolean) (SweepResult :type Hit%20Result%20Structure%20%28by%20ref%29))
  (Utilities|Casting|CastToBP_Char OtherActor)
  (bind _asvr_game_mode (Utilities|Casting|CastToVR_GameMode (Game|GetGameMode)))
  (Default|AddSpawner _asvr_game_mode)
  (Utilities|FlowControl|Delay 2.0)
  (Actor|DestroyActor))

(event Custom|SpawnItem
  (bind _itemarea (Variables|Default|GetItemArea))
  (bind _returnvalue (AddComponent|AddChildActorComponent false (Math|Conversions|ToTransform(Vector) (Math|Random|RandomPointinBoundingBox (Variables|/Script/Engine.SceneComponent|GetRelativeLocation _itemarea) (Variables|/Script/Engine.BoxComponent|GetBoxExtent _itemarea)))))
  (Transformation|SetWorldScale3D _returnvalue "4.000000,4.000000,4.000000"))

(event EventBeginPlay
  (for _index (range 0 5)
    (CallFunction|SpawnItem)))

(event Collision|EventActorBeginOverlap
  (params (OtherActor :type Actor%20Object%20Reference)))

(event EventTick
  (params (DeltaSeconds :type Float%20%28single-precision%29)))

(fn ConstructionScript)

(fn GetAttachTransform
  (return (Transformation|GetWorldTransform (Variables|Default|GetAttachPoint))))